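; Poster actor that grows larger each time the player pawn leaves its Box trigger.
; BeginPlay resets the Poster component to unit scale and stores that in NowScale.
; Each end overlap by the player adds a fixed step to X and Z and sets Y scale to zero, saving the result so growth accumulates without limit.
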(event `self.ReceiveBeginPlay`
  (`SceneComponent.SetRelativeScale3D` (`self.Poster`) (1.0 1.0 1.0))
  (set `self.Now Scale` (1.0 1.0 1.0)))

(event `self.Box.OnComponentEndOverlap`
  (params (OverlappedComponent :type "PrimitiveComponent Object Reference") (OtherActor :type "Actor Object Reference") (OtherComp :type "PrimitiveComponent Object Reference") (OtherBodyIndex :type Integer))
  (bind (_now_scale_x _now_scale_y _now_scale_z) (`KismetMathLibrary.BreakVector` (`self.Now Scale`)))
  (bind _returnvalue (+ _now_scale_z 1.5))
  (bind _returnvalue_2 (+ _now_scale_x 1.5))
  (if (== OtherActor (`GameplayStatics.GetPlayerPawn` 0))
    (`SceneComponent.SetRelativeScale3D` (`self.Poster`) (`KismetMathLibrary.MakeVector` _returnvalue_2 0.0 _returnvalue))
    (set `self.Now Scale` (`KismetMathLibrary.MakeVector` _returnvalue_2 0.0 _returnvalue))))

(fn `UserConstructionScript`)